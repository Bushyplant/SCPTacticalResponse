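; BP_LightShootingRange is a shooting range light actor that switches twelve point lights between normal and dimmed states.
; On BeginPlay it caches the intensity and color of the first PointLight as the shared defaults.
; Interface events drive the switch: turn-on applies those defaults to all twelve lights, while turn-off sets them to a fixed low intensity and dark grey instead of disabling them.
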(event `self.ReceiveBeginPlay`
  (bind _pointlight (`self.PointLight`))
  (set `self.PointLightIntensityDefault` (`LightComponentBase.Intensity` _pointlight))
  (set `self.PointLightColourDefault` (`LightComponentBase.GetLightColor` _pointlight)))

(event `/Game/_main/Interactables/BPI_Lights.BPI_TurnOnLight`
  (bind _pointlight (`self.PointLight`))
  (`LightComponent.SetIntensity` _pointlight (`self.PointLightIntensityDefault`))
  (`LightComponent.SetIntensity` (`self.PointLight6`) (`self.PointLightIntensityDefault`))
  (`LightComponent.SetIntensity` (`self.PointLight4`) (`self.PointLightIntensityDefault`))
  (`LightComponent.SetIntensity` (`self.PointLight3`) (`self.PointLightIntensityDefault`))
  (`LightComponent.SetIntensity` (`self.PointLight2`) (`self.PointLightIntensityDefault`))
  (`LightComponent.SetIntensity` (`self.PointLight1`) (`self.PointLightIntensityDefault`))
  (`LightComponent.SetIntensity` (`self.PointLight7`) (`self.PointLightIntensityDefault`))
  (`LightComponent.SetIntensity` (`self.PointLight8`) (`self.PointLightIntensityDefault`))
  (`LightComponent.SetIntensity` (`self.PointLight9`) (`self.PointLightIntensityDefault`))
  (`LightComponent.SetIntensity` (`self.PointLight10`) (`self.PointLightIntensityDefault`))
  (`LightComponent.SetIntensity` (`self.PointLight11`) (`self.PointLightIntensityDefault`))
  (`LightComponent.SetIntensity` (`self.PointLight5`) (`self.PointLightIntensityDefault`))
  (`LightComponent.SetLightColor` _pointlight (`self.PointLightColourDefault`) true)
  (`LightComponent.SetLightColor` (`self.PointLight7`) (`self.PointLightColourDefault`) true)
  (`LightComponent.SetLightColor` (`self.PointLight8`) (`self.PointLightColourDefault`) true)
  (`LightComponent.SetLightColor` (`self.PointLight9`) (`self.PointLightColourDefault`) true)
  (`LightComponent.SetLightColor` (`self.PointLight10`) (`self.PointLightColourDefault`) true)
  (`LightComponent.SetLightColor` (`self.PointLight11`) (`self.PointLightColourDefault`) true)
  (`LightComponent.SetLightColor` (`self.PointLight5`) (`self.PointLightColourDefault`) true)
  (`LightComponent.SetLightColor` (`self.PointLight1`) (`self.PointLightColourDefault`) true)
  (`LightComponent.SetLightColor` (`self.PointLight2`) (`self.PointLightColourDefault`) true)
  (`LightComponent.SetLightColor` (`self.PointLight3`) (`self.PointLightColourDefault`) true)
  (`LightComponent.SetLightColor` (`self.PointLight4`) (`self.PointLightColourDefault`) true)
  (`LightComponent.SetLightColor` (`self.PointLight6`) (`self.PointLightColourDefault`) true))

(event `/Game/_main/Interactables/BPI_Lights.BPI_TurnOffLight`
  (bind _pointlight (`self.PointLight`))
  (`LightComponent.SetIntensity` _pointlight 100.0)
  (`LightComponent.SetIntensity` (`self.PointLight6`) 100.0)
  (`LightComponent.SetIntensity` (`self.PointLight4`) 100.0)
  (`LightComponent.SetIntensity` (`self.PointLight3`) 100.0)
  (`LightComponent.SetIntensity` (`self.PointLight2`) 100.0)
  (`LightComponent.SetIntensity` (`self.PointLight1`) 100.0)
  (`LightComponent.SetIntensity` (`self.PointLight5`) 100.0)
  (`LightComponent.SetIntensity` (`self.PointLight11`) 100.0)
  (`LightComponent.SetIntensity` (`self.PointLight10`) 100.0)
  (`LightComponent.SetIntensity` (`self.PointLight9`) 100.0)
  (`LightComponent.SetIntensity` (`self.PointLight8`) 100.0)
  (`LightComponent.SetIntensity` (`self.PointLight7`) 100.0)
  (`LightComponent.SetLightColor` _pointlight (struct :`R` 0.140625 :`G` 0.140625 :`B` 0.140625 :`A` 1.0) true)
  (`LightComponent.SetLightColor` (`self.PointLight6`) (struct :`R` 0.140625 :`G` 0.140625 :`B` 0.140625 :`A` 1.0) true)
  (`LightComponent.SetLightColor` (`self.PointLight4`) (struct :`R` 0.140625 :`G` 0.140625 :`B` 0.140625 :`A` 1.0) true)
  (`LightComponent.SetLightColor` (`self.PointLight3`) (struct :`R` 0.140625 :`G` 0.140625 :`B` 0.140625 :`A` 1.0) true)
  (`LightComponent.SetLightColor` (`self.PointLight2`) (struct :`R` 0.140625 :`G` 0.140625 :`B` 0.140625 :`A` 1.0) true)
  (`LightComponent.SetLightColor` (`self.PointLight1`) (struct :`R` 0.140625 :`G` 0.140625 :`B` 0.140625 :`A` 1.0) true)
  (`LightComponent.SetLightColor` (`self.PointLight5`) (struct :`R` 0.140625 :`G` 0.140625 :`B` 0.140625 :`A` 1.0) true)
  (`LightComponent.SetLightColor` (`self.PointLight11`) (struct :`R` 0.140625 :`G` 0.140625 :`B` 0.140625 :`A` 1.0) true)
  (`LightComponent.SetLightColor` (`self.PointLight10`) (struct :`R` 0.140625 :`G` 0.140625 :`B` 0.140625 :`A` 1.0) true)
  (`LightComponent.SetLightColor` (`self.PointLight9`) (struct :`R` 0.140625 :`G` 0.140625 :`B` 0.140625 :`A` 1.0) true)
  (`LightComponent.SetLightColor` (`self.PointLight8`) (struct :`R` 0.140625 :`G` 0.140625 :`B` 0.140625 :`A` 1.0) true)
  (`LightComponent.SetLightColor` (`self.PointLight7`) (struct :`R` 0.140625 :`G` 0.140625 :`B` 0.140625 :`A` 1.0) true))

(fn `UserConstructionScript`)