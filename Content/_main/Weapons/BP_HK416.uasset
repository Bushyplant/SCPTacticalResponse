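; BP_HK416 is a weapon actor that motion controllers can grab and release, with main and secondary grip roles.
; Grab inside the main grip sphere attaches the SKAR4 mesh to that controller using the Grippoint socket; otherwise the controller becomes the secondary grip.
; With both controllers set, Tick feeds look-at and controller rotation values into SetActorLocation.
; Release compares against SecondaryGripCollision, not SecondaryGripController, and magazine collision is unused.
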(event `/Game/_main/BI_Grab.Release`
  (params (MotionController :type "MotionControllerComponent Object Reference"))
  (`|ExecutionSequence`
    (:`then_0`
      (if (== MotionController (`self.MainGripController`))
        (set `self.MainGripController` null)
        (set `self.SecondaryGripCollision` null)
        (`self.K2_DetachFromActor` "KeepWorld" "KeepWorld" "KeepWorld" :!label _label)))
    (:`then_1`
      (if (== MotionController (`self.SecondaryGripCollision`))
        (set `self.SecondaryGripCollision` null)
        (`self.MainGripCollision`
          (:`then`
            (`self.K2_SetActorRelativeTransform` (`SceneComponent.GetSocketTransform` (`self.SK_AR4`) "Grippoint" "RTS_Actor")))
          (:`else`
            (goto _label)))))))

(event `/Game/_main/BI_Grab.Grab`
  (params (MotionController :type "MotionControllerComponent Object Reference"))
  (bind _maingripcollision (`self.MainGripCollision`))
  (if (<= (`KismetMathLibrary.Vector_Distance` (`SceneComponent.K2_GetComponentLocation` _maingripcollision) (`SceneComponent.K2_GetComponentLocation` MotionController)) (`SphereComponent.SphereRadius` _maingripcollision))
    (bind _output_get (set `self.MainGripController` MotionController))
    (`SceneComponent.K2_AttachToComponent` (`self.SK_AR4`) _output_get "None" "SnapToTarget" "SnapToTarget" "KeepWorld" true)
    (`self.K2_SetActorRelativeTransform` (`SceneComponent.GetSocketTransform` (`self.SK_AR4`) "Grippoint" "RTS_Actor"))
    (elif true
      (set `self.SecondaryGripController` MotionController))))

(event `self.ReceiveTick`
  (params (DeltaSeconds :type "Float (single-precision)"))
  (bind _maingripcontroller (`self.MainGripController`))
  (bind (_returnvalue_roll _returnvalue_pitch) (`KismetMathLibrary.BreakRotator` (`SceneComponent.K2_GetComponentRotation` _maingripcontroller)))
  (bind (_returnvalue_roll_2 _returnvalue_pitch_2 _returnvalue_yaw) (`KismetMathLibrary.BreakRotator` (`KismetMathLibrary.ComposeRotators` (`KismetMathLibrary.FindLookAtRotation` (`SceneComponent.K2_GetComponentLocation` _maingripcontroller) (`SceneComponent.K2_GetComponentLocation` (`self.SecondaryGripController`))) (struct :`Yaw` -90.0))))
  (if (and (`KismetSystemLibrary.IsValid` (`self.MainGripController`)) (`KismetSystemLibrary.IsValid` (`self.SecondaryGripController`)))
    (`self.K2_SetActorLocation` (`KismetMathLibrary.MakeVector` (* _returnvalue_pitch_2 -1.0) _returnvalue_pitch _returnvalue_yaw))))

(fn `UserConstructionScript`)