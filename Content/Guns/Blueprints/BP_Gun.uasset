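; VR gun actor with hand-specific input, a draggable slide, magazine insertion and release, and firing mode switching.
; Timers interpolate slide and magazine motion; racking ejects and chambers rounds with sound and haptics, and can reattach the hand mesh to the slide.
; Trigger pressure animates hand and trigger, firing past a threshold only in Semi Automatic.
; Shots line-trace from the barrel for decals, impact effects, damage or impulse, and randomize recoil values.
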(event `self.ReceiveBeginPlay`
  (if (not (`self.HasFiringModes`))
    (`KismetSystemLibrary.PrintString` "GUN HAS NO FIRING MODES" true true (struct :`R` 0.6 :`A` 1.0))))

(event `self.MainGrabComponent.OnGrabbed`
  (params (MotionController :type "MotionControllerComponent Object Reference"))
  ;[1 1 1] Main Grab
  (`self.Motion Controller`
    (:`then`
      (`EnhancedInputSubsystemInterface.RemoveMappingContext` (pcsubsystem `EnhancedInputLocalPlayerSubsystem` (`GameplayStatics.GetPlayerController` 0)) (select `bool` (`|EnumEquality` (`/Game/VRTemplate/Blueprints/GrabComponent.GetHeldByHand` (`self.MainGrabComponent`)) "Right") :`false` "/Game/VRTemplate/Input/IMC_Weapon_Right.IMC_Weapon_Right" :`true` "/Game/VRTemplate/Input/IMC_Weapon_Left.IMC_Weapon_Left" :!type "InputMappingContext Object Reference") (struct))
      (set `self.Motion Controller` null))
    (:`else`
      _))
  (set `self.Motion Controller` MotionController)
  (bind _holdinghandanim (`self.GetHoldingHandAnim`))
  (set `self.Holding Hand Anim` _holdinghandanim)
  (`self.EnableInput` (`GameplayStatics.GetPlayerController` 0))
  (`EnhancedInputSubsystemInterface.AddMappingContext` (pcsubsystem `EnhancedInputLocalPlayerSubsystem` (`GameplayStatics.GetPlayerController` 0)) (select `bool` (`|EnumEquality` (`/Game/VRTemplate/Blueprints/GrabComponent.GetHeldByHand` (`self.MainGrabComponent`)) "Left") :`false` "/Game/VRTemplate/Input/IMC_Weapon_Right.IMC_Weapon_Right" :`true` "/Game/VRTemplate/Input/IMC_Weapon_Left.IMC_Weapon_Left" :!type "InputMappingContext Object Reference") 1 (struct)))

(event `self.MainGrabComponent.OnDropped`
  ;[1 1 1] Main Grab
  (`self.DisableInput` (`GameplayStatics.GetPlayerController` 0))
  (`EnhancedInputSubsystemInterface.RemoveMappingContext` (pcsubsystem `EnhancedInputLocalPlayerSubsystem` (`GameplayStatics.GetPlayerController` 0)) (select `bool` (`|EnumEquality` (`/Game/VRTemplate/Blueprints/GrabComponent.GetHeldByHand` (`self.MainGrabComponent`)) "Left") :`false` "/Game/VRTemplate/Input/IMC_Weapon_Right.IMC_Weapon_Right" :`true` "/Game/VRTemplate/Input/IMC_Weapon_Left.IMC_Weapon_Left" :!type "InputMappingContext Object Reference") (struct)))

(event `EnhancedInput|/Game/VRTemplate/Input/Actions/IA_Gun_Shoot_Left`
  (params (ActionValue :type "Float (double-precision)") (ElapsedSeconds :type "Float (double-precision)") (TriggeredSeconds :type "Float (double-precision)") (InputAction :type "InputAction Object Reference" :default "/Game/VRTemplate/Input/Actions/IA_Gun_Shoot_Left.IA_Gun_Shoot_Left"))
  (:`Triggered`
    (switch `/Game/Guns/GrapEnums/ENUM_FireModes` (`self.CurrentFiringMode`)
      (:`NewEnumerator1`
        _)
      (:`NewEnumerator2`
        _)
      (:`NewEnumerator3`
        _))
    (bind _output_get (set `self.ActionValueLeft` ActionValue))
    (set `/Game/_main/Hands/ABP_Hand.TriggerPressedValue` _output_get (`self.Holding Hand Anim`))
    (`SceneComponent.K2_SetRelativeRotation` (`self.Trigger`) (`KismetMathLibrary.RLerp` (struct) (`self.TriggerFinalPosRotation`) (`self.ActionValueLeft`)) false false)
    (if (> (`self.ActionValueLeft`) (`self.FireThreshold`))
      (if (`self.HasFiringModes`) :!label _label
        (switch `/Game/Guns/GrapEnums/ENUM_FireModes` (`self.CurrentFiringMode`)
          (:`NewEnumerator1`
            (if (not (`self.TriggerPressed`))
              (set `self.TriggerPressed` true)
              (`self.SingleShot`)))))
      (else
        (set `self.TriggerPressed` false :!label _label_2))))
  (:`Canceled`
    (switch `/Game/Guns/GrapEnums/ENUM_FireModes` (`self.CurrentFiringMode`) :!label _label_3
      (:`NewEnumerator1`
        _)
      (:`NewEnumerator2`
        _)
      (:`NewEnumerator3`
        _))
    (set `self.ActionValueLeft` 0.0)
    (set `/Game/_main/Hands/ABP_Hand.TriggerPressedValue` 0.0 (`self.Holding Hand Anim`))
    (goto _label_2))
  (:`Completed`
    (goto _label_3)))

(event `EnhancedInput|/Game/VRTemplate/Input/Actions/IA_Gun_Shoot_Right`
  (params (ActionValue :type "Float (double-precision)") (ElapsedSeconds :type "Float (double-precision)") (TriggeredSeconds :type "Float (double-precision)") (InputAction :type "InputAction Object Reference" :default "/Game/VRTemplate/Input/Actions/IA_Gun_Shoot_Right.IA_Gun_Shoot_Right"))
  (:`Triggered`
    (switch `/Game/Guns/GrapEnums/ENUM_FireModes` (`self.CurrentFiringMode`)
      (:`NewEnumerator1`
        _)
      (:`NewEnumerator2`
        _)
      (:`NewEnumerator3`
        _))
    (bind _output_get (set `self.ActionValueRight` ActionValue))
    (set `/Game/_main/Hands/ABP_Hand.TriggerPressedValue` _output_get (`self.Holding Hand Anim`))
    (`SceneComponent.K2_SetRelativeRotation` (`self.Trigger`) (`KismetMathLibrary.RLerp` (struct) (`self.TriggerFinalPosRotation`) (`self.ActionValueRight`)) false false)
    (if (> (`self.ActionValueRight`) (`self.FireThreshold`))
      (goto _label)
      (else
        (goto _label_2))))
  (:`Canceled`
    (switch `/Game/Guns/GrapEnums/ENUM_FireModes` (`self.CurrentFiringMode`) :!label _label_4
      (:`NewEnumerator1`
        _)
      (:`NewEnumerator2`
        _)
      (:`NewEnumerator3`
        _))
    (set `self.ActionValueRight` 0.0)
    (set `/Game/_main/Hands/ABP_Hand.TriggerPressedValue` 0.0 (`self.Holding Hand Anim`))
    (goto _label_2))
  (:`Completed`
    (goto _label_4)))

(event `self.CurlGrabComponent.OnGrabbed`
  (params (MotionController :type "MotionControllerComponent Object Reference"))
  ;[0 0 0 1 48] Grabbing Slider
  (`self.AttachHandToSlide` MotionController)
  ;;[0 0 0 1 32] Play Slider Grabbed Sound Cue
  (`GameplayStatics.PlaySoundAtLocation` (`self.SlideGrabbedSoundCue`) (`SceneComponent.K2_GetComponentLocation` (`self.SlideGrabCollision`)) (struct) 1.0 1.0 0.0 null null null null)
  ;;[0 0 0 1 32] Storing Intitial Offset Between MC & Handle
  (set `self.Intial Grab Offset` (`self.GetGrabOffsetBetweenMC&Slide`))
  (set `self.SliderReleased` false)
  (`KismetSystemLibrary.K2_SetTimerDelegate` (delegate `Interpolate Slide Movement`) 0.01 true) ; Setting timer for moving the slider while grabbed
)

(event `Interpolate Slide Movement`
  (bind _round (`self.Round`))
  (bind _returnvalue (`self.ClampSlideMovement` (`self.ChargingHandleMaxDistance`)))
  ;[0 0 0 1 48] Grabbing Slider
  (set `self.CurrentSlideOffset` _returnvalue) ; Current handle Pos
  (if (and (== _returnvalue (`self.ChargingHandleMaxDistance`)) (not (`self.ReachedLockedPosition?`)))
    ;;[0 0 0] Play Sound cue when Grabbing slide
    (set `self.ReachedLockedPosition?` true)
    (`GameplayStatics.PlaySoundAtLocation` (`self.SlideGrabbedSoundCue`) (`SceneComponent.K2_GetComponentLocation` (`self.SlideGrabCollision`)) (struct) 1.0 1.0 0.0 null null null null)
    ;;[0 0 0] Gun Communication Logic
    (bind _magazine (`self.Magazine`)
      (:`then`
        (if (`/Game/Guns/Blueprints/BP_Magazine.IsEmpty` _magazine)
          (set `self.Dryfire` true :!label _label)
          (set `self.BulletReadyToBeTaken` false)
          (else
            (set `self.Dryfire` false)
            (set `self.BulletReadyToBeTaken` true))))
      (:`else`
        (goto _label)))
    (if (`self.ChamberHasBullet`)
      (`self.InitiateBulletThrowAndSetRoundMeshInvis`))
    (`self.PlayHapticEffect` 0.8)
    (elif (`self.ReachedLockedPosition?`)
      (if (>= (`self.CurrentSlideOffset`) (+ (`self.ChargingHandleMaxDistance`) (`self.DistanceTotravelBackFromLockToGetBullet`)))
        (bind _magazine_2 (`self.Magazine`)
          (:`then`
            (if (`/Game/Guns/Blueprints/BP_Magazine.IsEmpty` _magazine_2)
              (`SceneComponent.SetVisibility` _round false false)
              (set `self.ChamberHasBullet` false)
              (else
                (`SceneComponent.SetVisibility` _round true false)
                (`/Game/Guns/Blueprints/BP_Magazine.RemoveRound` _magazine_2)
                (set `self.ChamberHasBullet` true)))
            (set `self.ReachedLockedPosition?` false))
          (:`else`
            _)))))
  ;;[0 0 0 1 32] Assigning Current Slide pos for handle
  (`SceneComponent.K2_SetRelativeLocation` (`self.Handle`) (`KismetMathLibrary.MakeVector` (`self.CurrentSlideOffset`)) false false))

(event `self.CurlGrabComponent.OnDropped`
  ;[0 0 0 1 50] Releasing the handle
  (`self.DetachHandFromSlide`) ; Detaching MC from Hand
  ;;[0 0 0] Clearing Out refs
  (set `self.SlideGrabMotionController` null)
  (set `self.SlideMotionControllerHandMesh` null)
  (`KismetSystemLibrary.K2_PauseTimer` null "Interpolate Slide Movement") ; Pausing Slider Movement and preparing to move it to orgin
  (if (<= (`self.CurrentSlideOffset`) (`self.OffsetToPlayReleaseSound`))
    ;;[0 0 0] Play Slide release Sound
    (`GameplayStatics.PlaySoundAtLocation` (`self.SlideReleaseSoundCue`) (`SceneComponent.K2_GetComponentLocation` (`self.Muzzel`)) (struct) 1.0 1.0 0.0 null null null null)
    (`self.PlayHapticEffectOnOpposideHand` 1.0))
  (set `self.SliderReleased` true)
  (`KismetSystemLibrary.K2_SetTimerDelegate` (delegate `ReturnSlideBack`) 0.01 true))

(event `ReturnSlideBack`
  ;[0 0 0 1 50] Releasing the handle
  (bind _hasreachedorigin (`self.InterpolateHandleToInitialPositionAndContinueOnceDone`)) ; Move Handle back to orgin/ return true if it came back
  (if _hasreachedorigin
    (`SceneComponent.K2_SetRelativeLocation` (`self.Handle`) (0.0 0.0 0.0) false false) ; Explicitty Assign Handle's location to 0
    (`KismetSystemLibrary.K2_PauseTimer` null "ReturnSlideBack") ; Stop return handle to orgin
    (set `self.CurrentSlideOffset` 0.0) ; Also Explicitity Set to 0
    (if (`self.ReachedLockedPosition?`)
      (bind _magazine (`self.Magazine`)
        (:`then`
          (if (`self.BulletReadyToBeTaken`)
            (if (`/Game/Guns/Blueprints/BP_Magazine.IsEmpty` _magazine)
              (if (`self.ChamberHasBullet`)
                (set `self.Dryfire` true :!label _label_2)
                (`SceneComponent.SetVisibility` (`self.Round`) false false)
                (set `self.ChamberHasBullet` false)
                (set `self.ReachedLockedPosition?` false :!label _label_3))
              (else
                (`/Game/Guns/Blueprints/BP_Magazine.RemoveRound` (`self.Magazine`))
                (`SceneComponent.SetVisibility` (`self.Round`) true false)
                (set `self.ChamberHasBullet` true)
                (goto _label_3)))
            (else
              (set `self.ReachedLockedPosition?` false :!label _label_4)
              (goto _label_2))))
        (:`else`
          (goto _label_4))))))

(event `self.MagazineCollision.OnComponentBeginOverlap`
  (params (OverlappedComponent :type "PrimitiveComponent Object Reference") (OtherActor :type "Actor Object Reference") (OtherComp :type "PrimitiveComponent Object Reference") (OtherBodyIndex :type Integer) (bFromSweep :type Boolean) (SweepResult :type "HitResult Structure (by ref)"))
  (bind _magazine (`self.Magazine`))
  (bind _curlgrabcomponent (`/Game/Guns/Blueprints/BP_Magazine.CurlGrabComponent` _magazine))
  ;[0 0 0 1 50] Inserting Magazine
  ;;[0 0 0 1 23] Check If We Don't Have Magazine And If We Overlap A magazine
  (`self.Magazine`
    (:`then`)
    (:`else`
      (bind _asbp_magazine (cast `/Game/Guns/Blueprints/BP_Magazine` OtherActor))
      ;;[0 0 0 1 23] Checking If Magazine And Gun Types Are Same and If Magazine Is Held
      (if (`|EnumEquality` (`/Game/Guns/Blueprints/BP_Magazine.MagType` _asbp_magazine) (`self.GunType`))
        (if (`/Game/VRTemplate/Blueprints/CurlGrabComponent.bIsHeld` (`/Game/Guns/Blueprints/BP_Magazine.CurlGrabComponent` _asbp_magazine))
          (bind _output_get (set `self.Magazine` _asbp_magazine))
          ;;[0 0 0 1 23] Turning The Physics Off Before Insertion
          (`PrimitiveComponent.SetSimulatePhysics` (`/Game/Guns/Blueprints/BP_Magazine.MagazineMesh` _output_get) false)
          (set `/Game/VRTemplate/Blueprints/CurlGrabComponent.bSimulateOnDrop` false (`/Game/Guns/Blueprints/BP_Magazine.CurlGrabComponent` _output_get))
          (`/Game/Guns/Blueprints/BP_Magazine.PlayInSound` _magazine)
          ;;[0 0 0 1 23] Explicitly Releasing Magazine
          (`/Game/VRTemplate/Blueprints/CurlGrabComponent.TryRelease` _curlgrabcomponent)
          (add `/Game/VRTemplate/Blueprints/CurlGrabComponent.OnGrabbed` _curlgrabcomponent (delegate `Simulate Magazine Physics On Dropped`)) ; Binding Event On Our Next Grab (Magazine Is Alaready In The Gun)
          (`KismetSystemLibrary.K2_SetTimerDelegate` (delegate `Smooth Attachment`) 0.01 true) ; Timer For Smooth Magazine Insertion
        )))))

(event `Smooth Attachment`
  ;[0 0 0 1 50] Inserting Magazine
  (bind _returnvalue (`self.SmoothMagazineAttachmentAndContinueOnceDone`)) ; Interpolation Of Magazine
  (if _returnvalue
    (`self.K2_AttachToComponent` (`self.Magazine`) (`self.GunMesh`) "Magazine" "SnapToTarget" "SnapToTarget" "KeepRelative" true)
    (`KismetSystemLibrary.K2_PauseTimer` null "Smooth Attachment") ; Stop Interpolating
  ))

(event `Simulate Magazine Physics On Dropped`
  (params (MotionController :type "MotionControllerComponent Object Reference"))
  (bind _curlgrabcomponent (`/Game/Guns/Blueprints/BP_Magazine.CurlGrabComponent` (`self.Magazine`)))
  ;[0 0 0 1 50] Inserting Magazine
  ;;[0 0 0 1 23] Happens On Next Grab (Magazine Is In The Gun)
  (set `/Game/VRTemplate/Blueprints/CurlGrabComponent.bSimulateOnDrop` true _curlgrabcomponent)
  (remove `/Game/VRTemplate/Blueprints/CurlGrabComponent.OnGrabbed` _curlgrabcomponent (delegate `Simulate Magazine Physics On Dropped`)) ; Unbind This Event To Avoid Not Simulating Physics After Drop Of The Magazine
  (set `self.Magazine` null))

(event `EnhancedInput|/Game/VRTemplate/Input/Actions/IA_SwitchGunMode_Left`
  (params (ActionValue :type Boolean) (ElapsedSeconds :type "Float (double-precision)") (TriggeredSeconds :type "Float (double-precision)") (InputAction :type "InputAction Object Reference" :default "/Game/VRTemplate/Input/Actions/IA_SwitchGunMode_Left.IA_SwitchGunMode_Left"))
  (:`Completed`
    (`self.SwitchGunMode` :!label _label)))

(event `EnhancedInput|/Game/VRTemplate/Input/Actions/IA_SwitchGunMode_Right`
  (params (ActionValue :type Boolean) (ElapsedSeconds :type "Float (double-precision)") (TriggeredSeconds :type "Float (double-precision)") (InputAction :type "InputAction Object Reference" :default "/Game/VRTemplate/Input/Actions/IA_SwitchGunMode_Right.IA_SwitchGunMode_Right"))
  (:`Completed`
    (goto _label)))

(event `EnhancedInput|/Game/VRTemplate/Input/Actions/IA_DropMag_Left`
  (params (ActionValue :type Boolean) (ElapsedSeconds :type "Float (double-precision)") (TriggeredSeconds :type "Float (double-precision)") (InputAction :type "InputAction Object Reference" :default "/Game/VRTemplate/Input/Actions/IA_DropMag_Left.IA_DropMag_Left"))
  (bind _curlgrabcomponent (`/Game/Guns/Blueprints/BP_Magazine.CurlGrabComponent` (`self.Magazine`)))
  (:`Completed`
    (bind _magazine (`self.Magazine` :!label _label_2)
      (:`then`
        (`/Game/Guns/Blueprints/BP_Magazine.PlayOutSound` _magazine)
        (bind _magazinemesh (`/Game/Guns/Blueprints/BP_Magazine.MagazineMesh` _magazine))
        (`SceneComponent.K2_DetachFromComponent` _magazinemesh "KeepWorld" "KeepWorld" "KeepWorld" true)
        (`PrimitiveComponent.SetSimulatePhysics` _magazinemesh true)
        (clear `/Game/VRTemplate/Blueprints/CurlGrabComponent.OnGrabbed` _curlgrabcomponent)
        (set `/Game/VRTemplate/Blueprints/CurlGrabComponent.bSimulateOnDrop` true _curlgrabcomponent)
        (set `self.Magazine` null))
      (:`else`))))

(event `EnhancedInput|/Game/VRTemplate/Input/Actions/IA_DropMag_Right`
  (params (ActionValue :type Boolean) (ElapsedSeconds :type "Float (double-precision)") (TriggeredSeconds :type "Float (double-precision)") (InputAction :type "InputAction Object Reference" :default "/Game/VRTemplate/Input/Actions/IA_DropMag_Right.IA_DropMag_Right"))
  (:`Completed`
    (goto _label_2)))

(fn `Apply Physics and Damage`
  (params (Seed :type Integer) (HitResult :type "HitResult Structure"))
  (bind (_bblockinghit _binitialoverlap _time _distance _location _impactpoint _normal _impactnormal _physmat _hitactor _hitcomponent _hitbonename _bonename) (`GameplayStatics.BreakHitResult` HitResult))
  (set `self.Seed` Seed)
  (if _bblockinghit
    (if (`KismetSystemLibrary.DoesImplementInterface` _hitactor "/Game/Guns/BPI_Damage.BPI_Damage_C")
      ;[1 0 0] Damage
      (message `/Game/Guns/BPI_Damage.BulletDamage` _hitactor (`self.Seed`) _bonename (* _impactnormal (/ (`self.ImpactForce`) 2.0)) (`self.DamageMultiplier`) (`GameplayStatics.GetPlayerPawn` 0))
      (return)
      (elif (`SceneComponent.IsSimulatingPhysics` _hitcomponent "None")
        (`PrimitiveComponent.AddImpulse` _hitcomponent (* _impactnormal (/ (`self.ImpactForce`) 2.0)) "None" false)
        (return)))))

(fn `AttachHandToSlide`
  (params (MotionController :type "MotionControllerComponent Object Reference"))
  (bind _output_get (set `self.SlideGrabMotionController` MotionController))
  (for _array_element (`SceneComponent.GetChildrenComponents` _output_get false)
    (bind _asb_mannequins_xr (cast `/Game/Characters/MannequinsXR/B_MannequinsXR` _array_element))
    (bind _output_get_2 (set `self.SlideMotionControllerHandMesh` _asb_mannequins_xr))
    (break))
  (if (`|EnumEquality` (`/Game/VRTemplate/Blueprints/CurlGrabComponent.GetHeldByHand` (`self.CurlGrabComponent`)) "Right")
    (`SceneComponent.K2_AttachToComponent` _output_get_2 (`self.SlideHard_R`) "None" "SnapToTarget" "SnapToTarget" "SnapToTarget" true)
    (else
      (`SceneComponent.K2_AttachToComponent` _output_get_2 (`self.SlideHard_L`) "None" "SnapToTarget" "SnapToTarget" "SnapToTarget" true)))
  (return))

(fn `BulletDefaultImpactDecals`
  (params (HitComponent :type "PrimitiveComponent Object Reference") (HitLocation :type "Vector Structure") (Normal :type "Vector Structure"))
  (bind _returnvalue (`GameplayStatics.SpawnDecalAttached` "/Game/Guns/Global/Materials/M_Bullet_decal.M_Bullet_decal" (2.0 2.0 2.0) HitComponent "None" HitLocation (`KismetMathLibrary.Conv_VectorToRotator` Normal) "KeepRelativeOffset" 10.0))
  (`/Engine/EditorBlueprintResources/StandardMacros.IsValid` _returnvalue
    (:`Is Valid`
      (`DecalComponent.SetFadeScreenSize` _returnvalue 0.001)
      (`DecalComponent.SetFadeIn` _returnvalue 0.0 0.01)
      (`DecalComponent.SetFadeOut` _returnvalue 15.0 15.0 false))))

(fn `ClampSlideMovement`
  (params (Min :type "Float (double-precision)"))
  (returns (ReturnValue :type "Float (double-precision)"))
  (bind _relativelocation_x (`KismetMathLibrary.BreakVector` (`SceneComponent.RelativeLocation` (`self.Handle`))))
  (bind _returnvalue_x (`KismetMathLibrary.BreakVector` (`KismetMathLibrary.InverseTransformLocation` (`SceneComponent.K2_GetComponentToWorld` (`self.Handle`)) (- (`SceneComponent.K2_GetComponentLocation` (`/Game/VRTemplate/Blueprints/CurlGrabComponent.MotionControllerRef` (`self.CurlGrabComponent`))) (`self.Intial Grab Offset`)))))
  (return (`KismetMathLibrary.FClamp` (+ _returnvalue_x _relativelocation_x) Min 0.0)))

(fn `DetachHandFromSlide`
  (bind _slidemotioncontrollerhandmesh (`self.SlideMotionControllerHandMesh`))
  (`SceneComponent.K2_AttachToComponent` (`self.SlideMotionControllerHandMesh`) (`self.SlideGrabMotionController`) "None" "SnapToTarget" "SnapToTarget" "SnapToTarget" true)
  (if (`|EnumEquality` (`/Game/VRTemplate/Blueprints/CurlGrabComponent.GetHeldByHand` (`self.CurlGrabComponent`)) "Right")
    (`SceneComponent.K2_AddRelativeRotation` _slidemotioncontrollerhandmesh (struct :`Pitch` -53.0 :`Yaw` -13.5 :`Roll` 106.8) false false)
    (else
      (`SceneComponent.K2_AddRelativeRotation` _slidemotioncontrollerhandmesh (struct :`Pitch` -53.7 :`Yaw` 2.64 :`Roll` 265.9) false false)
      (`SceneComponent.SetRelativeScale3D` _slidemotioncontrollerhandmesh (* (`SceneComponent.RelativeScale3D` _slidemotioncontrollerhandmesh) (1.0 -1.0 1.0)))))
  (`SceneComponent.K2_SetRelativeLocation` _slidemotioncontrollerhandmesh (-6.2 0.1 5.6) false false)
  (return))

(fn `GetGrabOffsetBetweenMC&Slide`
  (returns (IntialOffset :type "Vector Structure"))
  (return (- (`SceneComponent.K2_GetComponentLocation` (`/Game/VRTemplate/Blueprints/CurlGrabComponent.MotionControllerRef` (`self.CurlGrabComponent`))) (`SceneComponent.K2_GetComponentLocation` (`self.Handle`)))))

(fn `GetHoldingHandAnim`
  (returns (HoldingHandAnim :type "/Game/_main/Hands/ABP_Hand Object Reference"))
  (bind _maingrabcomponent (`self.MainGrabComponent`))
  (if (`|EnumEquality` (`/Game/VRTemplate/Blueprints/GrabComponent.GetHeldByHand` _maingrabcomponent) "Left")
    (return (`/Game/VRTemplate/Blueprints/GrabComponent.LeftHandAnim` _maingrabcomponent))
    (else
      (return (`/Game/VRTemplate/Blueprints/GrabComponent.RightHandAnim` _maingrabcomponent)))))

(fn `GunLocationAndDirection`
  (params (Distance :type "Float (double-precision)"))
  (returns (Location :type "Vector Structure") (Direction :type "Vector Structure"))
  (bind _gunmesh (`self.GunMesh`))
  (bind _returnvalue (`KismetMathLibrary.SelectVector` (`SceneComponent.GetSocketLocation` _gunmesh "SilencerBarrel") (`SceneComponent.GetSocketLocation` _gunmesh "Barrel") (`self.SilencerAttached`)))
  (return _returnvalue (+ _returnvalue (* (`KismetMathLibrary.GetForwardVector` (`SceneComponent.GetSocketRotation` _gunmesh "Barrel")) Distance))))

(fn `HasFiringModes`
  (returns (`Has At Least 1 Firing Mode` :type Boolean))
  (return (> (`KismetArrayLibrary.Array_Length` (`self.FiringModes`)) 0)))

(fn `ImpactDecals`
  (params (Hit :type "HitResult Structure"))
  (bind (_bblockinghit _binitialoverlap _time _distance _location _impactpoint _normal _impactnormal _physmat _hitactor _hitcomponent) (`GameplayStatics.BreakHitResult` Hit))
  (switch `EPhysicalSurface` (`PhysicalMaterial.SurfaceType` _physmat)
    (:`SurfaceType_Default`
      (`self.BulletDefaultImpactDecals` _hitcomponent _impactpoint _normal))))

(fn `ImpactSoundsAndParticles`
  (params (Hit :type "HitResult Structure"))
  (bind (_bblockinghit _binitialoverlap _time _distance _location _impactpoint _normal _impactnormal _physmat) (`GameplayStatics.BreakHitResult` Hit))
  (bind _surfacetype (`PhysicalMaterial.SurfaceType` _physmat))
  (if _bblockinghit
    (`NiagaraFunctionLibrary.SpawnSystemAtLocation` (select `EPhysicalSurface` _surfacetype :`SurfaceType_Default` "/Game/Guns/Global/VFX/P_BulletImpact_default.P_BulletImpact_default" :!type "NiagaraSystem Object Reference") _impactpoint (`KismetMathLibrary.Conv_VectorToRotator` _impactnormal))
    (`GameplayStatics.SpawnSoundAtLocation` (select `EPhysicalSurface` _surfacetype :`SurfaceType_Default` "/Game/Guns/Global/Audio/Cue_Bullet_Impact_Default.Cue_Bullet_Impact_Default" :!type "SoundBase Object Reference") _impactpoint (struct) 2.0 1.0 0.0 "/Game/Guns/Global/Audio/BulletImpactAttenuation.BulletImpactAttenuation" null)))

(fn `InitiateBulletThrowAndSetRoundMeshInvis`
  (bind (_returnvalue_location _returnvalue_rotation _returnvalue_scale) (`KismetMathLibrary.BreakTransform` (`SceneComponent.K2_GetComponentToWorld` (`self.Round`))))
  (`NiagaraFunctionLibrary.SpawnSystemAtLocation` (`self.SlideRoundEjection`) _returnvalue_location _returnvalue_rotation _returnvalue_scale)
  (`SceneComponent.SetVisibility` (`self.Round`) false false)
  (return))

(fn `InterpolateHandleToInitialPositionAndContinueOnceDone`
  (returns (HasReachedOrigin :type Boolean))
  (bind _handle (`self.Handle`))
  (bind _relativelocation_x (`KismetMathLibrary.BreakVector` (`SceneComponent.RelativeLocation` _handle)))
  (bind _returnvalue (`KismetMathLibrary.FInterpTo` _relativelocation_x 0.0 (* (`GameplayStatics.GetWorldDeltaSeconds`) (`self.SliderSnapToOriginSpeedMultiplyer`)) 0.4))
  (`SceneComponent.K2_SetRelativeLocation` _handle (`KismetMathLibrary.MakeVector` _returnvalue) false false)
  (return (`KismetMathLibrary.NearlyEqual_FloatFloat` _returnvalue 0.0 0.01)))

(fn `LineTraceFromBarrel`
  (params (Start :type "Vector Structure") (End :type "Vector Structure"))
  (returns (OutHit :type "HitResult Structure"))
  (bind _outhit (`KismetSystemLibrary.LineTraceSingle` Start End "TraceTypeQuery1"))
  (return _outhit))

(fn `LineTraceImpactDecalsAndRandomizingRecoilAndSoundsAndDamage`
  (bind (_location _direction) (`self.GunLocationAndDirection` 2000.0))
  (bind _outhit (`self.LineTraceFromBarrel` _location _direction))
  (`self.ImpactDecals` _outhit)
  (`self.RandomizingRecoil`)
  (bind _randomseed (`self.RandomDamageSeed`))
  (`self.ImpactSoundsAndParticles` _outhit)
  (`self.Apply Physics and Damage` _randomseed _outhit)
  (return))

(fn `PlayHapticEffect`
  (params (Scale :type "Float (double-precision)"))
  (`PlayerController.PlayHapticEffect` (`GameplayStatics.GetPlayerController` 0) (`self.HapticEffect`) (`/Game/VRTemplate/Blueprints/CurlGrabComponent.GetHeldByHand` (`self.CurlGrabComponent`)) Scale false)
  (return))

(fn `PlayHapticEffectOnOpposideHand`
  (params (Scale :type "Float (double-precision)"))
  (bind _returnvalue (`GameplayStatics.GetPlayerController` 0))
  (bind _hapticeffect (`self.HapticEffect`))
  (if (`|EnumEquality` (`/Game/VRTemplate/Blueprints/CurlGrabComponent.GetHeldByHand` (`self.CurlGrabComponent`)) "Left")
    (`PlayerController.PlayHapticEffect` _returnvalue _hapticeffect "Right" 1.0 false)
    (else
      (`PlayerController.PlayHapticEffect` _returnvalue _hapticeffect "Left" Scale false)))
  (return))

(fn `RandomDamageSeed`
  (returns (RandomSeed :type Integer))
  (return (`KismetMathLibrary.RandomIntegerInRange` 0 100)))

(fn `RandomizingRecoil`
  ;[0 0 0] Extreme Valuves if gun is grabbed with only one hand
  (set `self.RandomRecoilY` (`KismetMathLibrary.RandomFloatInRange` -0.65 0.65))
  (set `self.RandomRecoilX` (`KismetMathLibrary.RandomFloatInRange` 0.0 0.75)))

(fn `SingleShot`
  (bind _sliderreleased (`self.SliderReleased`))
  (`self.Magazine`
    (:`then`
      (if (`self.ChamberHasBullet`)
        (if (`/Game/Guns/Blueprints/BP_Magazine.IsEmpty` (`self.Magazine`))
          (if _sliderreleased :!label _label
            (`self.LineTraceImpactDecalsAndRandomizingRecoilAndSoundsAndDamage`)
            (`self.StoreGunRotationAndLocation`)
            (else
              (if (`self.Dryfire`) :!label _label_2
                (`GameplayStatics.PlaySoundAtLocation` (`self.DryFireSoundCue`) (`SceneComponent.K2_GetComponentLocation` (`self.Trigger`)) (struct) 1.0 1.0 0.0 null null null null)
                (set `self.Dryfire` false)
                (else
                  (`GameplayStatics.PlaySoundAtLocation` (`self.EmptyTriggerSoundCue`) (`SceneComponent.K2_GetComponentLocation` (`self.Trigger`)) (struct) 1.0 1.0 0.0 null null null null)))))
          (elif _sliderreleased
            (`/Game/Guns/Blueprints/BP_Magazine.RemoveRound` (`self.Magazine`))
            (`self.LineTraceImpactDecalsAndRandomizingRecoilAndSoundsAndDamage`)
            (`self.StoreGunRotationAndLocation`)
            (else
              (goto _label_2))))
        (else
          (goto _label_2))))
    (:`else`
      (if (`self.ChamberHasBullet`)
        (goto _label)
        (else
          (goto _label_2))))))

(fn `SmoothMagazineAttachmentAndContinueOnceDone`
  (returns (ReturnValue :type Boolean))
  (bind _magazine (`self.Magazine`))
  (bind _returnvalue (`SceneComponent.GetSocketLocation` (`self.GunMesh`) "Magazine"))
  (bind _returnvalue_2 (`KismetMathLibrary.VInterpTo` (`SceneComponent.K2_GetComponentLocation` (`/Game/Guns/Blueprints/BP_Magazine.MagazineMesh` _magazine)) _returnvalue (* (`GameplayStatics.GetWorldDeltaSeconds`) (`self.MagSnapToOriginSpeedMultiplyer`)) 1.0))
  (`SceneComponent.K2_SetRelativeLocation` (`Actor.RootComponent` _magazine) _returnvalue_2 false false)
  (return (== _returnvalue _returnvalue_2 :`ErrorTolerance` 0.01)))

(fn `StoreGunRotationAndLocation`
  (bind _gunmesh (`self.GunMesh`))
  (set `self.Relative Location` (`SceneComponent.RelativeLocation` _gunmesh))
  (set `self.Relative Rotation` (`SceneComponent.RelativeRotation` _gunmesh))
  (return))

(fn `SwitchGunMode`
  (if (`self.HasFiringModes`)
    (if (== (`self.CurrentFiringModeIndex`) (- (`KismetArrayLibrary.Array_Length` (`self.FiringModes`)) 1))
      (set `self.CurrentFiringMode` (`|GetArrayItem` (`self.FiringModes`)))
      (set `self.CurrentFiringModeIndex` 0)
      (else
        (bind _result (`/Engine/EditorBlueprintResources/StandardMacros.IncrementInt` (`self.CurrentFiringModeIndex`))
          (:`  `
            (bind _output_get (set `self.CurrentFiringModeIndex` _result))
            (set `self.CurrentFiringMode` (`|GetArrayItem` (`self.FiringModes`) _output_get))))))
    (`KismetSystemLibrary.PrintString` (`|GetEnumeratorNameAsString` (`self.CurrentFiringMode`)))
    (else
      (`KismetSystemLibrary.PrintString` "GUN HAS NO FIRING MODES" true true (struct :`R` 1.0 :`G` 0.010268 :`A` 1.0)))))

(fn `UserConstructionScript`)