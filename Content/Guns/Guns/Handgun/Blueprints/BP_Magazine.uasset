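; Handgun magazine actor that tracks its round count and shows the cartridges inside as instanced static meshes.
; When a round mesh override is set, the construction script procedurally stacks instances in single or staggered columns, with width and height taper and curvature.
; RemoveRound decrements the count, removes an instance through MulticastRemoveCartridgeMeshInstance and updates the empty flag.
; Helpers report remaining rounds and play magazine in and out sounds.
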(fn `HasRounds`
  (returns (ReturnValue :type Boolean))
  (return (!= (`self.Rounds`) 0)))

(fn `IsEvenNumber`
  (params (Number :type Integer))
  (returns (ReturnValue :type Boolean))
  (return (== (mod Number 2) 0)))

(fn `MulticastRemoveCartridgeMeshInstance`
  (`InstancedStaticMeshComponent.RemoveInstance` (`self.ISM_Rounds`) (`self.Rounds`)))

(fn `PlayInSound`
  (`GameplayStatics.PlaySoundAtLocation` (`self.MagInSound`) (`SceneComponent.K2_GetComponentLocation` (`self.MagazineMesh`)) (struct) 1.0 1.0 0.0 null null null null))

(fn `PlayOutSound`
  (`GameplayStatics.PlaySoundAtLocation` (`self.MagOutSound`) (`SceneComponent.K2_GetComponentLocation` (`self.MagazineMesh`)) (struct) 1.0 1.0 0.0 null null null null))

(fn `RemoveRound`
  (returns (Output_Get :type Boolean))
  (if (not (`self.IsEmpty`))
    (bind _output_get (set `self.Rounds` (- (`self.Rounds`) 1)))
    (`self.MulticastRemoveCartridgeMeshInstance`))
  (if (== _output_get 0)
    (set `self.IsEmpty` true)
    (else
      (bind _output_get_2 (set `self.IsEmpty` false))))
  (return _output_get_2))

(fn `UserConstructionScript`
  (bind _index (`self.Index`))
  (bind _heigthoffsettaperstart (`self.HeigthOffsetTaperStart`))
  (bind _radius (`self.Radius`))
  (bind _returnvalue (`KismetMathLibrary.Conv_IntToDouble` _heigthoffsettaperstart))
  (bind _returnvalue_2 (* _radius -1.0))
  (bind _returnvalue_3 (`KismetMathLibrary.Clamp` (- (`self.Index`) (`self.CurveStart`)) 0 (`self.Rounds`)))
  (bind _overrideroundmesh (`self.OverrideRoundMesh`)
    (:`then`
      (`StaticMeshComponent.SetStaticMesh` (`self.ISM_Rounds`) _overrideroundmesh)
      (for _index_2 (range (+ (`self.Rounds`) 1))
        (set `self.Index` _index_2)
        (`InstancedStaticMeshComponent.AddInstance` (`self.ISM_Rounds`) (`KismetMathLibrary.MakeTransform` (+ (+ (`self.StartLocation`) (`KismetMathLibrary.GreaterGreater_VectorRotator` (`KismetMathLibrary.MakeVector` 0.0 (`KismetMathLibrary.SelectFloat` 0.0 (/ (`KismetMathLibrary.SelectFloat` _radius _returnvalue_2 (== (`self.IsEvenNumber` _index_2) (`self.FlipStacking`))) (+ (`self.WidthOffset`) (* (`KismetMathLibrary.Clamp` (- (`self.WidthTaperOffsetStart`) (`self.Index`)) 0 (`self.Rounds`)) (`self.WidthOffsetTaper`)))) (`self.SingleStacking`)) (+ (* (* (`self.Index`) _returnvalue_2) (`self.HeightOffset`)) (* (`self.HeightOffsetTaper`) (`KismetMathLibrary.SelectFloat` (`KismetMathLibrary.MapRangeClamped` (`KismetMathLibrary.Conv_IntToDouble` _index) 0.0 _returnvalue _returnvalue) 0.0 (< _index _heigthoffsettaperstart))))) (`KismetMathLibrary.MakeRotator` 0.0 (* _returnvalue_3 (`self.CurveStrength`))))) (`KismetMathLibrary.MakeVector` (* _returnvalue_3 (`self.CurveSharpness`)))) (`KismetMathLibrary.MakeRotator` 0.0 (* (`self.Rotation`) (`KismetMathLibrary.Conv_IntToDouble` _returnvalue_3))) (`KismetMathLibrary.Conv_DoubleToVector` (`self.Scale`))) false)))
    (:`else`)))