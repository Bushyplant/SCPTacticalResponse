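; Killhouse level actor with a movable wall and a set of point lights that can be switched between lit and dimmed.
; Entrance and exit collision overlaps snap the wall to one of two fixed world rotations, with no check on the overlapping actor.
; BeginPlay caches the first light's intensity and colour, which BPITurnonLight restores to all lights.
; BPITurnOffLight dims them to grey rather than off, though PointLight4 keeps its colour.
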(event `self.ExitColision.OnComponentBeginOverlap`
  (params (OverlappedComponent :type "PrimitiveComponent Object Reference") (OtherActor :type "Actor Object Reference") (OtherComp :type "PrimitiveComponent Object Reference") (OtherBodyIndex :type Integer) (bFromSweep :type Boolean) (SweepResult :type "HitResult Structure (by ref)"))
  (`SceneComponent.K2_SetWorldRotation` (`self.MOVABLEWALL`) (struct :`Yaw` 300.0) false false))

(event `self.EntranceCollision.OnComponentBeginOverlap`
  (params (OverlappedComponent :type "PrimitiveComponent Object Reference") (OtherActor :type "Actor Object Reference") (OtherComp :type "PrimitiveComponent Object Reference") (OtherBodyIndex :type Integer) (bFromSweep :type Boolean) (SweepResult :type "HitResult Structure (by ref)"))
  (`SceneComponent.K2_SetWorldRotation` (`self.MOVABLEWALL`) (struct :`Yaw` 220.0) false false))

(event `self.ReceiveBeginPlay`
  (bind _pointlight (`self.PointLight`))
  (set `self.PointLightIntensityDefault` (`LightComponentBase.Intensity` _pointlight))
  (set `self.PointLightColourDefault` (`LightComponentBase.GetLightColor` _pointlight)))

(event `/Game/_main/Interactables/BPI_Lights.BPI_TurnOnLight`
  (`LightComponent.SetIntensity` (`self.PointLight`) (`self.PointLightIntensityDefault`))
  (`LightComponent.SetIntensity` (`self.PointLight5`) (`self.PointLightIntensityDefault`))
  (`LightComponent.SetIntensity` (`self.PointLight3`) (`self.PointLightIntensityDefault`))
  (`LightComponent.SetIntensity` (`self.PointLight2`) (`self.PointLightIntensityDefault`))
  (`LightComponent.SetIntensity` (`self.PointLight1`) (`self.PointLightIntensityDefault`))
  (`LightComponent.SetIntensity` (`self.PointLight4`) (`self.PointLightIntensityDefault`))
  (`LightComponent.SetIntensity` (`self.PointLight10`) (`self.PointLightIntensityDefault`))
  (`LightComponent.SetIntensity` (`self.PointLight9`) (`self.PointLightIntensityDefault`))
  (`LightComponent.SetIntensity` (`self.PointLight6`) (`self.PointLightIntensityDefault`))
  (`LightComponent.SetIntensity` (`self.PointLight7`) (`self.PointLightIntensityDefault`))
  (`LightComponent.SetIntensity` (`self.PointLight8`) (`self.PointLightIntensityDefault`))
  (`LightComponent.SetLightColor` (`self.PointLight6`) (`self.PointLightColourDefault`) true)
  (`LightComponent.SetLightColor` (`self.PointLight7`) (`self.PointLightColourDefault`) true)
  (`LightComponent.SetLightColor` (`self.PointLight8`) (`self.PointLightColourDefault`) true)
  (`LightComponent.SetLightColor` (`self.PointLight9`) (`self.PointLightColourDefault`) true)
  (`LightComponent.SetLightColor` (`self.PointLight10`) (`self.PointLightColourDefault`) true)
  (`LightComponent.SetLightColor` (`self.PointLight4`) (`self.PointLightColourDefault`) true)
  (`LightComponent.SetLightColor` (`self.PointLight1`) (`self.PointLightColourDefault`) true)
  (`LightComponent.SetLightColor` (`self.PointLight2`) (`self.PointLightColourDefault`) true)
  (`LightComponent.SetLightColor` (`self.PointLight3`) (`self.PointLightColourDefault`) true)
  (`LightComponent.SetLightColor` (`self.PointLight5`) (`self.PointLightColourDefault`) true)
  (`LightComponent.SetLightColor` (`self.PointLight`) (`self.PointLightColourDefault`) true))

(event `/Game/_main/Interactables/BPI_Lights.BPI_TurnOffLight`
  (bind _pointlight (`self.PointLight`))
  (`LightComponent.SetIntensity` _pointlight 100.0)
  (`LightComponent.SetIntensity` (`self.PointLight5`) 100.0)
  (`LightComponent.SetIntensity` (`self.PointLight3`) 100.0)
  (`LightComponent.SetIntensity` (`self.PointLight2`) 100.0)
  (`LightComponent.SetIntensity` (`self.PointLight1`) 100.0)
  (`LightComponent.SetIntensity` (`self.PointLight4`) 100.0)
  (`LightComponent.SetIntensity` (`self.PointLight10`) 100.0)
  (`LightComponent.SetIntensity` (`self.PointLight9`) 100.0)
  (`LightComponent.SetIntensity` (`self.PointLight8`) 100.0)
  (`LightComponent.SetIntensity` (`self.PointLight7`) 100.0)
  (`LightComponent.SetIntensity` (`self.PointLight6`) 100.0)
  (`LightComponent.SetLightColor` _pointlight (struct :`R` 0.140625 :`G` 0.140625 :`B` 0.140625 :`A` 1.0) true)
  (`LightComponent.SetLightColor` (`self.PointLight5`) (struct :`R` 0.140625 :`G` 0.140625 :`B` 0.140625 :`A` 1.0) true)
  (`LightComponent.SetLightColor` (`self.PointLight3`) (struct :`R` 0.140625 :`G` 0.140625 :`B` 0.140625 :`A` 1.0) true)
  (`LightComponent.SetLightColor` (`self.PointLight2`) (struct :`R` 0.140625 :`G` 0.140625 :`B` 0.140625 :`A` 1.0) true)
  (`LightComponent.SetLightColor` (`self.PointLight1`) (struct :`R` 0.140625 :`G` 0.140625 :`B` 0.140625 :`A` 1.0) true)
  (`LightComponent.SetLightColor` (`self.PointLight10`) (struct :`R` 0.140625 :`G` 0.140625 :`B` 0.140625 :`A` 1.0) true)
  (`LightComponent.SetLightColor` (`self.PointLight9`) (struct :`R` 0.140625 :`G` 0.140625 :`B` 0.140625 :`A` 1.0) true)
  (`LightComponent.SetLightColor` (`self.PointLight8`) (struct :`R` 0.140625 :`G` 0.140625 :`B` 0.140625 :`A` 1.0) true)
  (`LightComponent.SetLightColor` (`self.PointLight7`) (struct :`R` 0.140625 :`G` 0.140625 :`B` 0.140625 :`A` 1.0) true)
  (`LightComponent.SetLightColor` (`self.PointLight6`) (struct :`R` 0.140625 :`G` 0.140625 :`B` 0.140625 :`A` 1.0) true))

(fn `UserConstructionScript`)